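; Player pawn that rotates grabbed objects and toggles an on-screen Terminal widget for text input.
; Holding right mouse steps the Grabber's hit actor roll through a self-calling Delay loop, resetting rotation near a full turn; release calls SetNumberOfDone.
; Tab shows or hides the Terminal, created at BeginPlay, along with the mouse cursor.
; The widget's event passes user input to FindText and prints the returned result.
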(event `self.ReceiveBeginPlay`
  (bind _returnvalue (`|CreateWidget` "/Game/Blueprints/Terminal.Terminal_C"))
  (set `self.myVal` _returnvalue))

(event `RotateObject`
  (bind __actorhit (`Grabber._actorHit` (`self.Grabber`)))
  (bind _returnvalue_roll (`KismetMathLibrary.BreakRotator` (`self.K2_GetActorRotation` __actorhit)))
  (bind _returnvalue (+ _returnvalue_roll 5.0))
  ;[1 1 1] Rotate Grabbed Object
  (`KismetSystemLibrary.Delay` 0.01)
  (if (`self.HoldRotate`)
    (`/Engine/EditorBlueprintResources/StandardMacros.IsValid` __actorhit
      (:`Is Valid`
        (if (>= _returnvalue 359.0)
          (`self.K2_SetActorRotation` __actorhit (`KismetMathLibrary.MakeRotator` 0.0) false)
          (else
            (`self.K2_SetActorRotation` __actorhit (`KismetMathLibrary.MakeRotator` _returnvalue) false)))
        (`self.RotateObject`)))))

(event `Key|RightMouseButton`
  (params (Key :type "Key Structure"))
  ;[1 1 1] Input from the user to rotate
  (:`Pressed`
    (set `self.HoldRotate` true)
    (`self.RotateObject`))
  (:`Released`
    (set `self.HoldRotate` false)
    (`Grabber.SetNumberOfDone` (`self.Grabber`))
    (`KismetSystemLibrary.PrintString` (`KismetStringLibrary.Conv_IntToString` (`Grabber.printVar` (`self.Grabber`))))))

(event `Key|Tab`
  (params (Key :type "Key Structure"))
  (bind _returnvalue (`GameplayStatics.GetPlayerController` 0))
  (bind _myval (`self.myVal`))
  (:`Pressed`
    (`/Engine/EditorBlueprintResources/StandardMacros.FlipFlop`
      (:`A`
        (`/Engine/EditorBlueprintResources/StandardMacros.IsValid` _myval
          (:`Is Valid`
            (`UserWidget.AddToViewport` _myval 0)
            (set `PlayerController.bShowMouseCursor` true _returnvalue)
            (add `/Game/Blueprints/Terminal.Event1` _myval (delegate `Event`)))))
      (:`B`
        (`Widget.RemoveFromParent` _myval)
        (set `PlayerController.bShowMouseCursor` false _returnvalue)))))

(event `Event`
  (bind _findtext (`self.FindText`))
  (`FindText.OnInput` _findtext (`/Game/Blueprints/Terminal.InputFromUser` (`self.myVal`)))
  (bind _returnvalue (`FindText.ReturnInput` _findtext))
  (`KismetSystemLibrary.PrintString` _returnvalue))

(fn `UserConstructionScript`)