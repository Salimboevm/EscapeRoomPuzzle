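; BP_Menu is a main menu actor that shows a MainMenu widget and moves the player's view between linked menu actors.
; On BeginPlay it binds the widget's TransitionToMenu dispatcher, whose index selects a target from LinkedMenus.
; A transition disables this actor's collision, enables the target's, and eases the player's view to the target with a timed blend.
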(event `self.ReceiveBeginPlay`
  (bind _asmain_menu (cast `/Game/Blueprints/MainMenu/Widgets/MainMenu` (`WidgetComponent.GetUserWidgetObject` (`self.Widget`))))
  (add `/Game/Blueprints/MainMenu/Widgets/Main.TransitionToMenu` _asmain_menu (delegate `TransitionBetweenMenus`)))

(event `TransitionBetweenMenus`
  (params (Index :type Integer))
  (if (`KismetArrayLibrary.Array_IsValidIndex` (`self.LinkedMenus`) Index)
    (`self.TransitionToThis` (`|GetArrayItem` (`self.LinkedMenus`) Index))))

(event `TransitionToThis`
  (params (`New Menu` :type "/Game/Blueprints/MainMenu/BP_Menu Object Reference"))
  (`self.SetActorEnableCollision` false)
  (`self.SetActorEnableCollision` `New Menu` true)
  (`PlayerController.SetViewTargetWithBlend` (`GameplayStatics.GetPlayerController` 0) `New Menu` 2.0 "VTBlend_EaseInOut" 2.0 false))

(fn `UserConstructionScript`)